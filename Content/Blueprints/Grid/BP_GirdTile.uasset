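; Grid tile actor that displays its ground type and its hover, selection and path states for a pathfinding grid.
; After a brief BeginPlay delay it scales to the grid's tile size and passes grid and index to its W_GridTile widget.
; Cursor events update the tile and notify BpGrid.
; SetTileColor layers these states into material parameters, while debug events tint open and closed set tiles.
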(event `self.ReceiveBeginPlay`
  (`KismetSystemLibrary.Delay` 0.01)
  (`self.SetTileColor`)
  (`self.SetTileSize`)
  (`self.SetTileVariables`))

(event `self.StaticMesh.OnBeginCursorOver`
  (params (TouchedComponent :type "PrimitiveComponent Object Reference"))
  (`self.StartOverTile`)
  (`/Game/Blueprints/Grid/BP_Grid.NewTileOvered` (`self.bp_Grid`) self))

(event `self.StaticMesh.OnEndCursorOver`
  (params (TouchedComponent :type "PrimitiveComponent Object Reference"))
  (`/Game/Blueprints/Grid/BP_Grid.NewTileOvered` (`self.bp_Grid`) null))

(event `StartOverTile`
  (set `self.bIsOvered` true)
  (`self.SetTileColor`))

(event `EndOverTile`
  (set `self.bIsOvered` false)
  (`self.SetTileColor`))

(event `self.StaticMesh.OnClicked`
  (params (TouchedComponent :type "PrimitiveComponent Object Reference") (ButtonPressed :type "Key Structure"))
  (`self.SelectTile`)
  (`/Game/Blueprints/Grid/BP_Grid.NewTileSelected` (`self.bp_Grid`) self))

(event `SelectTile`
  (set `self.bIsSelected` true)
  (`self.SetTileColor`))

(event `DeselectTile`
  (set `self.bIsSelected` false)
  (`self.SetTileColor`))

(event `Event_IsInPath`
  (params (`bIs in Path` :type Boolean))
  (set `self.bIsInPath` `bIs in Path`)
  (`self.SetTileColor`))

(event `DebugEvent_OpenSet`
  (`MeshComponent.SetVectorParameterValueOnMaterials` (`self.StaticMesh`) "TileColor" (`KismetMathLibrary.Conv_LinearColorToVector` (struct :`R` 0.354221 :`G` 1.0 :`B` 0.277083 :`A` 1.0))))

(event `DebugEvent_CloseSet`
  (`MeshComponent.SetVectorParameterValueOnMaterials` (`self.StaticMesh`) "TileColor" (`KismetMathLibrary.Conv_LinearColorToVector` (struct :`R` 1.0 :`G` 0.459574 :`B` 0.047752 :`A` 1.0))))

(fn `GetTileData`
  (returns (Value :type "/Game/Blueprints/Grid/Structure_Tiles Structure"))
  (return (`BlueprintMapLibrary.Map_Find` (`/Game/Blueprints/Grid/BP_Grid.Tiles` (`self.bp_Grid`)) (`self.Index`))))

(fn `SetTileColor`
  (locals (Color :type "LinearColor Structure"))
  (bind _value_groundtype (break `/Game/Blueprints/Grid/Structure_Tiles` (`self.GetTileData`)))
  (`|ExecutionSequence`
    (:`then_0`
      (switch `/Game/Blueprints/Grid/GroundType` _value_groundtype
        (:`NewEnumerator4`
          (set `local.Color` (struct :`R` 0.836151 :`G` 1.0 :`B` 0.580587 :`A` 1.0)))
        (:`NewEnumerator0`
          (set `local.Color` (struct :`R` 0.896269 :`G` 0.514918 :`B` 0.701102 :`A` 1.0)))
        (:`NewEnumerator1`
          (set `local.Color` (struct :`R` 0.752942 :`G` 0.194618 :`B` 0.274677 :`A` 1.0)))
        (:`NewEnumerator2`
          (set `local.Color` (struct :`R` 1.0 :`B` 0.029557 :`A` 1.0)))
        (:`NewEnumerator3`
          (set `local.Color` (struct :`R` 0.04375 :`G` 0.04375 :`B` 0.04375 :`A` 1.0)))))
    (:`then_1`
      (if (`self.bIsSelected`)
        (`MeshComponent.SetScalarParameterValueOnMaterials` (`self.StaticMesh`) "blsSelect" 1.0)
        (else
          (`MeshComponent.SetScalarParameterValueOnMaterials` (`self.StaticMesh`) "blsSelect" 0.0))))
    (:`then_2`
      (if (`self.bIsOvered`)
        (set `local.Color` (* (`local.Color`) 3.0))))
    (:`then_3`
      (if (`self.bIsInPath`)
        (set `local.Color` (struct :`R` 0.225607 :`G` 0.670908 :`B` 0.922917 :`A` 1.0))))
    (:`then_4`
      (`MeshComponent.SetVectorParameterValueOnMaterials` (`self.StaticMesh`) "TileColor" (`KismetMathLibrary.Conv_LinearColorToVector` (`local.Color`))))))

(fn `SetTileSize`
  (bind _staticmesh (`self.StaticMesh`))
  (bind (_returnvalue_x _returnvalue_y) (`KismetMathLibrary.BreakVector` (* (`SceneComponent.K2_GetComponentScale` _staticmesh) (/ (`/Game/Blueprints/Grid/BP_Grid.TileSize` (`self.bp_Grid`)) 50.0))))
  (`SceneComponent.SetWorldScale3D` _staticmesh (`KismetMathLibrary.MakeVector` _returnvalue_x _returnvalue_y 1.0)))

(fn `SetTileVariables`
  (bind _asw_grid_tile (cast `/Game/Blueprints/Grid/W_GridTile` (`WidgetComponent.GetUserWidgetObject` (`self.Widget`))))
  (set `/Game/Blueprints/Grid/W_GridTile.grid` (`self.bp_Grid`) _asw_grid_tile)
  (set `/Game/Blueprints/Grid/W_GridTile.girdIndex` (`self.Index`) _asw_grid_tile))

(fn `UserConstructionScript`)