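; Player controller that tracks the selected unit and relays movement paths to it.
; A new selection event deselects the previous valid unit and stores the new one, while a new path event tells the selected unit to move along that path.
; The R key uses a FlipFlop to alternately hide and show all Bp_Basic actors.
; A transform-to-selected-unit node is left unconnected and never runs.
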(event `self.ReceiveTick`
  (params (DeltaSeconds :type "Float (single-precision)")))

(event `Key|R`
  (params (Key :type "Key Structure"))
  (:`Pressed`
    (`/Engine/EditorBlueprintResources/StandardMacros.FlipFlop`
      (:`A`
        (bind _outactors (`GameplayStatics.GetAllActorsOfClass` "/Game/Blueprints/Grid/Obstacles/Bp_Basic.Bp_Basic_C"))
        (for _array_element _outactors
          (`self.SetActorHiddenInGame` _array_element true)))
      (:`B`
        (bind _outactors_2 (`GameplayStatics.GetAllActorsOfClass` "/Game/Blueprints/Grid/Obstacles/Bp_Basic.Bp_Basic_C"))
        (for _array_element_2 _outactors_2
          (`self.SetActorHiddenInGame` _array_element_2 false))))))

(event `Event_NewUnitSelected`
  (params (Unit :type "/Game/Blueprints/Controller/BP_Unit Object Reference"))
  (bind _selectedunit (`self.selectedUnit`))
  (`/Engine/EditorBlueprintResources/StandardMacros.IsValid` _selectedunit
    (:`Is Valid`
      (`/Game/Blueprints/Controller/BP_Unit.Event_Deselected` _selectedunit))
    (:`Is Not Valid`
      _))
  (set `self.selectedUnit` Unit))

(event `Event_NewPathAvailable`
  (params (path :type "Array of Vector2D Structure"))
  (bind _selectedunit (`self.selectedUnit`))
  (`/Engine/EditorBlueprintResources/StandardMacros.IsValid` _selectedunit
    (:`Is Valid`
      (`/Game/Blueprints/Controller/BP_Unit.Event_MoveAlongThePath` _selectedunit path))))

(fn `UserConstructionScript`)