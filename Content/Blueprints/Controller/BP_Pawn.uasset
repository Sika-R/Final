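; Player pawn that switches between free roaming and a fixed scene camera view.
; Tick adds consumed movement input straight to the actor location, without sweep or delta-time scaling, using capsule-relative axes.
; Space alternates a blended view target between the second CameraActor found at BeginPlay and the player controller, setting the Manyou (roam) flag.
; That flag gates look input and applying movement, but not accumulating movement input.
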(event `self.ReceiveBeginPlay`
  (bind _outactors (`GameplayStatics.GetAllActorsOfClass` "/Script/Engine.CameraActor"))
  (set `self.camera` (`|GetArrayItem` _outactors 1)))

(event `self.ReceiveTick`
  (params (DeltaSeconds :type "Float (single-precision)"))
  (if (`self.Manyou`)
    (bind _returnvalue (`self.ConsumeMovementInputVector`))
    (`self.K2_SetActorLocation` (+ _returnvalue (`self.K2_GetActorLocation` self)))))

(event `InputAxis|Turn` :overrideparent false
  (params (AxisValue :type "Float (single-precision)"))
  (if (`self.Manyou`)
    (`self.AddControllerYawInput` AxisValue)))

(event `InputAxis|LookUp` :overrideparent false
  (params (AxisValue :type "Float (single-precision)"))
  (if (`self.Manyou`)
    (`self.AddControllerPitchInput` AxisValue)))

(event `InputAxis|MoveForward` :overrideparent false
  (params (AxisValue :type "Float (single-precision)"))
  (`self.AddMovementInput` (`SceneComponent.GetForwardVector` (`self.Capsule`)) AxisValue))

(event `InputAxis|MoveRight` :overrideparent false
  (params (AxisValue :type "Float (single-precision)"))
  (`self.AddMovementInput` (`SceneComponent.GetRightVector` (`self.Capsule`)) AxisValue))

(event `Key|SpaceBar`
  (params (Key :type "Key Structure"))
  (bind _returnvalue (`GameplayStatics.GetPlayerController` 0))
  (:`Pressed`
    (`/Engine/EditorBlueprintResources/StandardMacros.FlipFlop`
      (:`A`
        (set `self.Manyou` false)
        (`PlayerController.SetViewTargetWithBlend` _returnvalue (`self.camera`) 1.0 "VTBlend_Linear" 0.5 false))
      (:`B`
        (set `self.Manyou` true)
        (`PlayerController.SetViewTargetWithBlend` _returnvalue _returnvalue 1.0 "VTBlend_Linear" 0.5 false)))))

(fn `UserConstructionScript`)