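; BP_Unit is a clickable unit on BP_Grid that can be selected and moved along tile paths.
; On BeginPlay it waits briefly, caches the player controller and grid, then snaps to the nearest tile.
; Clicks report selection changes to BP_PlayerController, while UnitOnThisTile updates tile occupancy in the grid's map.
; Movement rebuilds the grid's shared spline from the path and follows it with a timeline, flagging the grid as busy.
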(event `self.ReceiveBeginPlay`
  (`KismetSystemLibrary.Delay` 1.0)
  (bind _asbp_player_controller (cast `/Game/Blueprints/Controller/BP_PlayerController` (`GameplayStatics.GetPlayerController` 0)))
  (set `self.playerController` _asbp_player_controller)
  (bind _outactors (`GameplayStatics.GetAllActorsOfClass` "/Game/Blueprints/Grid/BP_Grid.BP_Grid_C"))
  (set `self.Grid` (`|GetArrayItem` _outactors))
  (`self.SetGridIndexAndSnapToLocation`))

(event `self.Cone.OnClicked`
  (params (TouchedComponent :type "PrimitiveComponent Object Reference") (ButtonPressed :type "Key Structure"))
  (`KismetSystemLibrary.Delay` 1e-05 :!label _label)
  (if (!= (`/Game/Blueprints/Controller/BP_PlayerController.selectedUnit` (`self.playerController`)) self)
    (`/Game/Blueprints/Controller/BP_PlayerController.Event_NewUnitSelected` (`self.playerController`) self)
    (`self.Event_Selected`)
    (else
      (`/Game/Blueprints/Controller/BP_PlayerController.Event_NewUnitSelected` (`self.playerController`) null))))

(event `self.Cone1.OnClicked`
  (params (TouchedComponent :type "PrimitiveComponent Object Reference") (ButtonPressed :type "Key Structure"))
  (goto _label))

(event `self.CapsuleComponent.OnClicked`
  (params (TouchedComponent :type "PrimitiveComponent Object Reference") (ButtonPressed :type "Key Structure"))
  (goto _label))

(event `Event_Selected`
  (`KismetSystemLibrary.PrintString` "Selected"))

(event `Event_Deselected`
  (`KismetSystemLibrary.PrintString` "Deselected"))

(event `Event_MoveAlongThePath`
  (params (path :type "Array of Vector2D Structure"))
  (bind _grid (`self.Grid`))
  (bind _path (`self.path`))
  (bind (_returnvalue_location _returnvalue_rotation _returnvalue_scale) (`KismetMathLibrary.BreakTransform` (`self.GetTransform` self)))
  (bind _spline (`/Game/Blueprints/Grid/BP_Grid.Spline` (`self.Grid`)))
  (set `self.path` path)
  (`KismetArrayLibrary.Array_Insert` _path (`self.gridIndex`))
  (`self.UnitOnThisTile` (`|GetArrayItem` _path (`KismetArrayLibrary.Array_LastIndex` _path)))
  (`SplineComponent.ClearSplinePoints` (`/Game/Blueprints/Grid/BP_Grid.Spline` (`self.Grid`)) true)
  (for _array_element (`self.path`)
    (bind _value (`BlueprintMapLibrary.Map_Find` (`/Game/Blueprints/Grid/BP_Grid.Tiles` (`self.Grid`)) _array_element))
    (`SplineComponent.AddSplinePoint` (`/Game/Blueprints/Grid/BP_Grid.Spline` (`self.Grid`)) (`KismetMathLibrary.MakeVector` (.x (`.WorldLocation_8_418E1AC54C19FA5ED69DE6A691756FAE` (break `/Game/Blueprints/Grid/Structure_Tiles` _value))) (.y (`.WorldLocation_8_418E1AC54C19FA5ED69DE6A691756FAE` (break `/Game/Blueprints/Grid/Structure_Tiles` _value))) (+ (.z (`.WorldLocation_8_418E1AC54C19FA5ED69DE6A691756FAE` (break `/Game/Blueprints/Grid/Structure_Tiles` _value))) (* (`CapsuleComponent.CapsuleHalfHeight` (`self.CapsuleComponent`)) 0.5))) "World" true))
  (set `/Game/Blueprints/Grid/BP_Grid.bIsAUnitMoving` true _grid)
  (`TimelineComponent.SetPlayRate` (`self.MoveAlongThePathTimeline`) 0.1)
  (bind (_direction _progession) (`Timeline|MoveAlongThePathTimeline`)
    (:`Update`
      (bind _returnvalue (* _progession (`SplineComponent.GetSplineLength` _spline)))
      (`self.K2_SetActorTransform` self (`KismetMathLibrary.MakeTransform` (`SplineComponent.GetLocationAtDistanceAlongSpline` _spline _returnvalue "World") (`SplineComponent.GetRotationAtDistanceAlongSpline` _spline _returnvalue "World") _returnvalue_scale) false false))
    (:`Finished`
      (set `/Game/Blueprints/Grid/BP_Grid.bIsAUnitMoving` false _grid))))

(fn `SetGridIndexAndSnapToLocation`
  (locals (closestDistance :type "Float (double-precision)") (closestIndex :type "Vector2D Structure"))
  (bind _tiles (`/Game/Blueprints/Grid/BP_Grid.Tiles` (`self.Grid`)))
  (set `local.closestDistance` 10000000000.0)
  (bind _keys (`BlueprintMapLibrary.Map_Keys` _tiles))
  (for _array_element _keys
    (bind _value (`BlueprintMapLibrary.Map_Find` _tiles _array_element))
    (bind _returnvalue (`KismetMathLibrary.VSize` (- (`.WorldLocation_8_418E1AC54C19FA5ED69DE6A691756FAE` (break `/Game/Blueprints/Grid/Structure_Tiles` _value)) (`self.K2_GetActorLocation` self))))
    (if (< _returnvalue (`local.closestDistance`))
      (set `local.closestDistance` _returnvalue)
      (set `local.closestIndex` (`.GridIndex_9_ABEA759C47F24E8708B148A2A44DCC71` (break `/Game/Blueprints/Grid/Structure_Tiles` _value)))))
  (`self.UnitOnThisTile` (`local.closestIndex`))
  (`self.K2_SetActorLocation` (`.WorldLocation_8_418E1AC54C19FA5ED69DE6A691756FAE` (break `/Game/Blueprints/Grid/Structure_Tiles` (`BlueprintMapLibrary.Map_Find` (`/Game/Blueprints/Grid/BP_Grid.Tiles` (`self.Grid`)) (`local.closestIndex`))))))

(fn `UnitOnThisTile`
  (params (gridIndex :type "Vector2D Structure"))
  (bind _gridindex (`self.gridIndex`))
  (bind _gridindex_2 (`self.gridIndex`))
  (bind _tiles (`/Game/Blueprints/Grid/BP_Grid.Tiles` (`self.Grid`)))
  (bind _tiles_2 (`/Game/Blueprints/Grid/BP_Grid.Tiles` (`self.Grid`)))
  (bind _value (`BlueprintMapLibrary.Map_Find` _tiles _gridindex))
  (bind _value_2 (`BlueprintMapLibrary.Map_Find` _tiles_2 _gridindex_2))
  (`BlueprintMapLibrary.Map_Add` _tiles_2 _gridindex_2 (make `/Game/Blueprints/Grid/Structure_Tiles` (break `/Game/Blueprints/Grid/Structure_Tiles` _value_2) (`.WorldLocation_8_418E1AC54C19FA5ED69DE6A691756FAE` (break `/Game/Blueprints/Grid/Structure_Tiles` _value_2)) (`.GridIndex_9_ABEA759C47F24E8708B148A2A44DCC71` (break `/Game/Blueprints/Grid/Structure_Tiles` _value_2)) (`.tileCost_24_D2C6D9974C3500A393A53582B7D7B33A` (break `/Game/Blueprints/Grid/Structure_Tiles` _value_2)) (`.FinalCost_12_63A43F184A71778E95967CBA45689F33` (break `/Game/Blueprints/Grid/Structure_Tiles` _value_2)) (`.costFromStart_22_771EBC78492E1E47F48E188FBA74F6E2` (break `/Game/Blueprints/Grid/Structure_Tiles` _value_2)) 0 (`.tileActor_25_67A705434CB16B943107F4A874B4CE43` (break `/Game/Blueprints/Grid/Structure_Tiles` _value_2)) (`.previousTile_28_5D6AE8A340F0A00924EC0AA4C40447BD` (break `/Game/Blueprints/Grid/Structure_Tiles` _value_2))))
  (set `self.gridIndex` gridIndex)
  (`BlueprintMapLibrary.Map_Add` _tiles _gridindex (make `/Game/Blueprints/Grid/Structure_Tiles` (break `/Game/Blueprints/Grid/Structure_Tiles` _value) (`.WorldLocation_8_418E1AC54C19FA5ED69DE6A691756FAE` (break `/Game/Blueprints/Grid/Structure_Tiles` _value)) (`.GridIndex_9_ABEA759C47F24E8708B148A2A44DCC71` (break `/Game/Blueprints/Grid/Structure_Tiles` _value)) (`.tileCost_24_D2C6D9974C3500A393A53582B7D7B33A` (break `/Game/Blueprints/Grid/Structure_Tiles` _value)) (`.FinalCost_12_63A43F184A71778E95967CBA45689F33` (break `/Game/Blueprints/Grid/Structure_Tiles` _value)) (`.costFromStart_22_771EBC78492E1E47F48E188FBA74F6E2` (break `/Game/Blueprints/Grid/Structure_Tiles` _value)) 0 (`.tileActor_25_67A705434CB16B943107F4A874B4CE43` (break `/Game/Blueprints/Grid/Structure_Tiles` _value)) (`.previousTile_28_5D6AE8A340F0A00924EC0AA4C40447BD` (break `/Game/Blueprints/Grid/Structure_Tiles` _value)) self)))

(fn `UserConstructionScript`)