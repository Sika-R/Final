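; BP_Location is a location actor in the StartMenu folder that resolves which grid tile it sits on.
; GetTileIndex runs a small, near zero-length sphere trace at the actor's position, casts the hit to BP_GirdTile and returns that tile with its index.
; The construction script runs a similar, larger complex trace but discards the result, and the event graph holds only empty default events.
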(fn `GetTileIndex`
  (params (Object :type "Object Object Reference"))
  (returns (Index :type "Vector2D Structure") (TargetTile :type "/Game/Blueprints/Grid/BP_GirdTile Object Reference"))
  (bind _returnvalue (`self.K2_GetActorLocation` self))
  (bind (_outhit _returnvalue_2) (`KismetSystemLibrary.SphereTraceSingle` :`Start` _returnvalue :`End` (+ _returnvalue 0.01) :`Radius` 10.0 :`TraceChannel` "TraceTypeQuery5" :`DrawTime` 10.0))
  (if _returnvalue_2
    (bind _asbp_gird_tile (cast `/Game/Blueprints/Grid/BP_GirdTile` (`.HitActor` (`GameplayStatics.BreakHitResult` _outhit))))
    (return (`/Game/Blueprints/Grid/BP_GirdTile.Index` _asbp_gird_tile) _asbp_gird_tile)))

(fn `UserConstructionScript`
  (bind _returnvalue (`self.K2_GetActorLocation` self))
  (`KismetSystemLibrary.SphereTraceSingle` :`Start` _returnvalue :`End` (+ _returnvalue 0.0001) :`Radius` 20.0 :`TraceChannel` "TraceTypeQuery5" :`bTraceComplex` true :`DrawTime` 10000000.0))