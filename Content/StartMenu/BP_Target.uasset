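; BP_Target is a clickable start menu hotspot that opens an info panel and moves the view to its own camera.
; StaticMesh events toggle mesh visibility for hover and press feedback.
; Clicking fills the DialogueText widget with Info and Facility, stops the Sphere's idle spin and blends to that camera.
; Clicking StaticMesh3 hides the panel and blends back to the second CameraActor found at BeginPlay.
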(event `self.ReceiveBeginPlay`
  (`SceneComponent.SetVisibility` (`self.StaticMesh1`) false false)
  (`SceneComponent.SetVisibility` (`self.StaticMesh2`) false false)
  (`SceneComponent.SetVisibility` (`self.StaticMesh3`) false false)
  (`SceneComponent.SetVisibility` (`self.StaticMesh4`) false false)
  (`SceneComponent.SetVisibility` (`self.Widget`) false false)
  (`SceneComponent.SetVisibility` (`self.StaticMesh`) true false)
  (bind _outactors (`GameplayStatics.GetAllActorsOfClass` "/Script/Engine.CameraActor"))
  (set `self.Camera1` (`|GetArrayItem` _outactors 1)))

(event `self.ReceiveTick`
  (params (DeltaSeconds :type "Float (single-precision)"))
  (if (not (`self.Open`))
    (`SceneComponent.K2_AddWorldRotation` (`self.Sphere`) (struct :`Yaw` 1.0) false false)))

(event `self.StaticMesh.OnClicked`
  (params (TouchedComponent :type "PrimitiveComponent Object Reference") (ButtonPressed :type "Key Structure"))
  (`SceneComponent.SetVisibility` (`self.StaticMesh1`) false false)
  (`SceneComponent.SetVisibility` (`self.StaticMesh2`) true false)
  (`SceneComponent.SetVisibility` (`self.StaticMesh3`) true false)
  (`SceneComponent.SetVisibility` (`self.Widget`) true false)
  (`SceneComponent.SetVisibility` (`self.StaticMesh4`) true false)
  (bind _asdialogue_text (cast `/Game/StartMenu/DialogueText` (`WidgetComponent.GetUserWidgetObject` (`self.Widget`))))
  (`/Game/StartMenu/DialogueText.UpdateInfo` _asdialogue_text (`self.Info`))
  (`/Game/StartMenu/DialogueText.UpdateFacililties` _asdialogue_text (`self.Facility`))
  (set `self.Open` true)
  (`SceneComponent.K2_SetWorldRotation` (`self.Sphere`) (struct :`Pitch` -90.0) false false)
  (`PlayerController.SetViewTargetWithBlend` (`GameplayStatics.GetPlayerController` 0) (`ActorComponent.GetOwner` (`self.Camera`)) 1.0 "VTBlend_Linear" 0.5 false))

(event `self.StaticMesh.OnReleased`
  (params (TouchedComponent :type "PrimitiveComponent Object Reference") (ButtonReleased :type "Key Structure"))
  (`SceneComponent.SetVisibility` (`self.StaticMesh2`) false false)
  (`SceneComponent.SetVisibility` (`self.StaticMesh1`) false false)
  (`SceneComponent.SetVisibility` (`self.StaticMesh1`) true false))

(event `self.StaticMesh.OnBeginCursorOver`
  (params (TouchedComponent :type "PrimitiveComponent Object Reference"))
  (`SceneComponent.SetVisibility` (`self.StaticMesh`) false false)
  (`SceneComponent.SetVisibility` (`self.StaticMesh2`) false false)
  (`SceneComponent.SetVisibility` (`self.StaticMesh1`) true false))

(event `self.StaticMesh.OnEndCursorOver`
  (params (TouchedComponent :type "PrimitiveComponent Object Reference"))
  (`SceneComponent.SetVisibility` (`self.StaticMesh1`) false false)
  (`SceneComponent.SetVisibility` (`self.StaticMesh2`) false false)
  (`SceneComponent.SetVisibility` (`self.StaticMesh`) true false))

(event `self.StaticMesh3.OnClicked`
  (params (TouchedComponent :type "PrimitiveComponent Object Reference") (ButtonPressed :type "Key Structure"))
  (if (`self.Open`)
    (`PlayerController.SetViewTargetWithBlend` (`GameplayStatics.GetPlayerController` 0) (`self.Camera1`) 1.0 "VTBlend_Linear" 0.0 false)
    (`SceneComponent.SetVisibility` (`self.StaticMesh3`) false false)
    (`SceneComponent.SetVisibility` (`self.Widget`) false false)
    (`SceneComponent.SetVisibility` (`self.StaticMesh4`) false false)
    (set `self.Open` false)))

(fn `UserConstructionScript`)